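; Enemy character that chases the player and fires projectiles, with a health bar facing the camera and an explosion on death.
; PawnSensing sightings trigger AIMoveTo, spawning a shot as each move is issued if shooting is allowed.
; SmokeDetector overlaps let smoking grenades temporarily blind it and slow grenades reduce speed and stop shooting.
; Projectile hits feed AnyDamage, as does a gas-damage event whose timer Tick re-arms every frame.
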(event OnComponentHit(HitBox)
  (params (HitComponent :type Primitive%20Component%20Object%20Reference) (OtherActor :type Actor%20Object%20Reference) (OtherComp :type Primitive%20Component%20Object%20Reference) (NormalImpulse :type Vector :default "0, 0, 0") (Hit :type Hit%20Result%20Structure%20%28by%20ref%29))
  ;[1 1 1] HitBox
  (bind _asbp_first_person_projectile (Utilities|Casting|CastToBP_FirstPersonProjectile OtherActor))
  (Game|Damage|ApplyDamage self 1e+01 0 _asbp_first_person_projectile))

(event OnSeePawn(PawnSensing)
  (params (Pawn :type Pawn%20Object%20Reference))
  ;[1 1 1] Move to player
  ;;[1 1 1] Can see?
  (Utilities|Casting|CastToBP_PlayerCharacter Pawn)
  (if (Variables|Default|GetCanSeePlayer?)
    (CallFunction|FollowPlayer)))

(event OnComponentBeginOverlap(SmokeDetector)
  (params (OverlappedComponent :type Primitive%20Component%20Object%20Reference) (OtherActor :type Actor%20Object%20Reference) (OtherComp :type Primitive%20Component%20Object%20Reference) (OtherBodyIndex :type Integer) (bFromSweep :type Boolean) (SweepResult :type Hit%20Result%20Structure%20%28by%20ref%29))
  ;[1 1 1] Move to player
  ;;[1 1 1] Blinded
  (Utilities|FlowControl|Sequence
    (:then_0
      (bind _asbp_grenade (Utilities|Casting|CastToBP_Grenade OtherActor))
      (if (Variables|/Game/Industry_Briefs_work/Blueprints/BP_Grenade.BP_Grenade_C|GetSmoke? _asbp_grenade)
        (Variables|Default|SetCanSeePlayer? false)
        (Rendering|SetVisibility (Variables|Default|Get?) true false)
        (Utilities|FlowControl|Delay 9.0)
        (Variables|Default|SetCanSeePlayer? true)
        (Rendering|SetVisibility (Variables|Default|Get?) false false)))
    (:then_1
      (bind _asbp_grenade_gas (Utilities|Casting|CastToBP_Grenade_Gas OtherActor))
      (if (Variables|/Game/Industry_Briefs_work/Blueprints/BP_Grenade_Gas.BP_Grenade_Gas_C|GetSmoke? _asbp_grenade_gas)
        (Variables|Default|SetCanSeePlayer? false)
        (Rendering|SetVisibility (Variables|Default|Get?) true false)
        (Utilities|FlowControl|Delay 9.0)
        (Variables|Default|SetCanSeePlayer? true)
        (Rendering|SetVisibility (Variables|Default|Get?) false false)))
    (:then_2
      (bind _asbp_grenade_quick (Utilities|Casting|CastToBP_Grenade_Quick OtherActor))
      (if (Variables|/Game/Industry_Briefs_work/Blueprints/BP_Grenade_Quick.BP_Grenade_Quick_C|GetSmoke? _asbp_grenade_quick)
        (Variables|Default|SetCanSeePlayer? false)
        (Rendering|SetVisibility (Variables|Default|Get?) true false)
        (Utilities|FlowControl|Delay 9.0)
        (Variables|Default|SetCanSeePlayer? true)
        (Rendering|SetVisibility (Variables|Default|Get?) false false)))
    (:then_3
      (bind _asbp_grenade_path_finding (Utilities|Casting|CastToBP_Grenade_PathFinding OtherActor))
      (if (Variables|/Game/Industry_Briefs_work/Blueprints/BP_Grenade_PathFinding.BP_Grenade_PathFinding_C|GetSmoke? _asbp_grenade_path_finding)
        (Variables|Default|SetCanSeePlayer? false)
        (Rendering|SetVisibility (Variables|Default|Get?) true false)
        (Utilities|FlowControl|Delay 9.0)
        (Variables|Default|SetCanSeePlayer? true)
        (Rendering|SetVisibility (Variables|Default|Get?) false false)))
    (:then_4
      (bind _asbp_grenade_slow (Utilities|Casting|CastToBP_Grenade_Slow OtherActor))
      (if (Variables|/Game/Industry_Briefs_work/Blueprints/BP_Grenade_Slow.BP_Grenade_Slow_C|GetExploded _asbp_grenade_slow)
        (Variables|/Script/Engine.CharacterMovementComponent|SetMaxWalkSpeed (Variables|Character|GetCharacterMovement) 3e+02)
        (Variables|Default|SetShoot? false)
        (Rendering|SetVisibility (Variables|Default|Get!) true false)
        (Utilities|FlowControl|Delay 4.5)
        (Variables|/Script/Engine.CharacterMovementComponent|SetMaxWalkSpeed (Variables|Character|GetCharacterMovement) 6e+02)
        (Variables|Default|SetShoot? true)
        (Rendering|SetVisibility (Variables|Default|Get!) false false)))))

(event Custom|FollowPlayer
  (bind _bulletref (Variables|Default|GetBulletREF))
  ;[1 1 1] Move to player
  (if (Variables|Default|GetCanSeePlayer?)
    (AI|AIMoveTo self "0, 0, 0" (Game|GetPlayerCharacter 0) 5.0 false
      (:then
        (Rendering|SetVisibility (Variables|Default|Get?) false false)
        (if (Variables|Default|GetShoot?)
          (Game|SpawnActorfromClass "/Game/FirstPerson/Blueprints/BP_EnemyProjectile.BP_EnemyProjectile_C" (Math|Transform|MakeTransform (Transformation|GetWorldLocation _bulletref) (Math|Rotator|MakeRotfromZ (Math|Vector|GetForwardVector _bulletref)) "0.200000,0.200000,0.200000") "Undefined" "MultiplyWithRoot" 0 0))))))

(event Custom|GasDamages
  ;[1 1 1] Gas damage
  (bind _returnvalue (Actor|GetActorOfClass "/Game/Industry_Briefs_work/Blueprints/BP_Grenade_Gas.BP_Grenade_Gas_C"))
  (Utilities|FlowControl|DoOnce false :!label _label
    (:Completed
      (Game|Damage|ApplyDamage self 2.0 0 _returnvalue)
      (Utilities|FlowControl|RetriggerableDelay 0.2)
      (goto _label Reset))))

(event EventTick
  (params (DeltaSeconds :type Float%20%28single-precision%29))
  (bind _returnvalue (Game|GetPlayerCameraManager 0))
  (bind _health (Variables|Default|GetHealth))
  (bind _returnvalue_2 (Transformation|GetWorldLocation _health))
  (bind _transformcomponent (Variables|/Script/Engine.PlayerCameraManager|GetTransformComponent _returnvalue))
  (bind _returnvalue_3 (Transformation|GetWorldLocation _transformcomponent))
  (bind _returnvalue_4 (Math|Rotator|FindLookatRotation _returnvalue_2 _returnvalue_3))
  ;[1 1 1] HealthBar
  (Utilities|FlowControl|Sequence
    (:then_0
      (bind _asai_health (Utilities|Casting|CastToAI_Health (UserInterface|GetWidget (Variables|Default|GetHealth))))
      (Progress|SetPercent (Variables|/Game/Industry_Briefs_work/Widgets/AI_Health.AI_Health_C|GetHealthbar _asai_health) (/ (Variables|Default|GetCurrentHealth) 1e+02))
      (Transformation|SetWorldRotation _health _returnvalue_4 false false)
      (Transformation|SetWorldRotation (Variables|Default|Get?) _returnvalue_4 false false)
      (Transformation|SetWorldRotation (Variables|Default|Get!) _returnvalue_4 false false))
    (:then_1
      ;[1 1 1] Gas damage
      (Utilities|Time|SetTimerbyEvent (delegate Custom|GasDamages) 1.0))))

(event Game|Damage|EventAnyDamage
  (params (Damage :type Float%20%28single-precision%29) (DamageType :type Damage%20Type%20Object%20Reference) (InstigatedBy :type Controller%20Object%20Reference) (DamageCauser :type Actor%20Object%20Reference))
  ;[1 1 1] Apply Damage
  (Variables|Default|SetCurrentHealth (Math|Float|Clamp(Float) (- (Variables|Default|GetCurrentHealth) Damage) 0.0 (Variables|Default|GetMaxHealth)))
  (if (== (Variables|Default|GetCurrentHealth) 0.0)
    (Effects|SpawnEmitteratLocation "/Game/Everything_Else/StarterContent/Particles/P_Explosion.P_Explosion" (Transformation|GetActorLocation))
    (Actor|DestroyActor)))

(fn ConstructionScript)