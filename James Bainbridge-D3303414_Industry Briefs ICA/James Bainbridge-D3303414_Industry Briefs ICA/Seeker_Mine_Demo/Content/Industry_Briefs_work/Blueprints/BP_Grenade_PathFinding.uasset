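; Smoke grenade actor that rolls along a navmesh path and bursts on contact with enemies.
; BeginPlay computes the path once to a stored location and starts a self-destruct timer.
; After a ground hit, and once DetectionField has found a BP_Enemy, Tick applies force toward successive path points.
; Trigger overlap briefly enables the Multiple collider, spawning smoke on overlapped enemies and at itself, then destroys the actor after a delay.
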(event OnComponentBeginOverlap(DetectionField)
  (params (OverlappedComponent :type Primitive%20Component%20Object%20Reference) (OtherActor :type Actor%20Object%20Reference) (OtherComp :type Primitive%20Component%20Object%20Reference) (OtherBodyIndex :type Integer) (bFromSweep :type Boolean) (SweepResult :type Hit%20Result%20Structure%20%28by%20ref%29))
  ;[1 1 1] Move towards enemy.
  (bind _asbp_enemy (Utilities|Casting|CastToBP_Enemy OtherActor))
  (Variables|Default|SetAs%20BP%20Enemy _asbp_enemy))

(event OnComponentBeginOverlap(Multiple?)
  (params (OverlappedComponent :type Primitive%20Component%20Object%20Reference) (OtherActor :type Actor%20Object%20Reference) (OtherComp :type Primitive%20Component%20Object%20Reference) (OtherBodyIndex :type Integer) (bFromSweep :type Boolean) (SweepResult :type Hit%20Result%20Structure%20%28by%20ref%29))
  ;[1 1 1] Multiple
  (bind _asbp_enemy (Utilities|Casting|CastToBP_Enemy OtherActor))
  (Effects|SpawnEmitteratLocation "/Game/Everything_Else/StarterContent/Particles/P_Smoke.P_Smoke" (Transformation|GetActorLocation _asbp_enemy))
  (Variables|Default|SetSmoke? true)
  (Audio|PlaySoundatLocation "/Game/Everything_Else/StarterContent/Audio/Smoke01.Smoke01" (Transformation|GetActorLocation) "0, 0, 0" 1.0 1.0 0.0 0 0 0 0)
  (Utilities|FlowControl|Delay 6.0)
  (Variables|Default|SetSmoke? false)
  (Actor|DestroyActor))

(event OnComponentHit(Sphere)
  (params (HitComponent :type Primitive%20Component%20Object%20Reference) (OtherActor :type Actor%20Object%20Reference) (OtherComp :type Primitive%20Component%20Object%20Reference) (NormalImpulse :type Vector :default "0, 0, 0") (Hit :type Hit%20Result%20Structure%20%28by%20ref%29))
  ;[1 1 1] Ground Detector
  (if (Utilities|Operators|EqualEqual (.ImpactNormal (Collision|BreakHitResult Hit)) "0.000000,0.000000,1.000000" 0.5)
    (Physics|SetSimulatePhysics (Variables|Default|GetGrenade) false)
    (Variables|Default|SetIs%20Grounded? true)))

(event OnComponentBeginOverlap(Trigger)
  (params (OverlappedComponent :type Primitive%20Component%20Object%20Reference) (OtherActor :type Actor%20Object%20Reference) (OtherComp :type Primitive%20Component%20Object%20Reference) (OtherBodyIndex :type Integer) (bFromSweep :type Boolean) (SweepResult :type Hit%20Result%20Structure%20%28by%20ref%29))
  ;[1 1 1] Basics
  (Utilities|Casting|CastToBP_Enemy OtherActor)
  (CallFunction|DoStuff))

(event Custom|Do%20stuff
  ;[1 1 1] Basics
  (Variables|Default|SetExploded true)
  (Collision|SetCollisionEnabled (Variables|Default|GetMultiple?) "QueryAndPhysics")
  (Utilities|FlowControl|Delay 1.0)
  (Collision|SetCollisionEnabled (Variables|Default|GetMultiple?) "NoCollision")
  (Effects|SpawnEmitteratLocation "/Game/Everything_Else/StarterContent/Particles/P_Smoke.P_Smoke" (Transformation|GetActorLocation))
  (Variables|Default|SetSmoke? true)
  (Audio|PlaySoundatLocation "/Game/Everything_Else/StarterContent/Audio/Smoke01.Smoke01" (Transformation|GetActorLocation) "0, 0, 0" 1.0 1.0 0.0 0 0 0 0)
  (Development|SetHiddeninGame (Variables|Default|GetGrenade) true false)
  (Utilities|FlowControl|Delay 6.0)
  (Variables|Default|SetSmoke? false)
  (Actor|DestroyActor))

(event EventBeginPlay
  ;[1 1 1] Multiple
  ;[1 1 1] Move towards enemy.
  (Utilities|FlowControl|Sequence
    (:then_0
      (Collision|SetCollisionEnabled (Variables|Default|GetMultiple?) "NoCollision")
      (if (not (Variables|Default|GetExploded))
        (Utilities|FlowControl|Delay 6.0)
        (Actor|DestroyActor)))
    (:then_1
      ;;[1 1 1] PathFinding
      (bind _returnvalue (Class|NavigationSystemV1|FindPathtoLocationSynchronously (Transformation|GetActorLocation) (Variables|Default|GetLast%20Index) self 0))
      (Variables|Default|SetPath%20Point%20Array (Variables|/Script/NavigationSystem.NavigationPath|GetPathPoints _returnvalue)))))

(event EventTick
  (params (DeltaSeconds :type Float%20%28single-precision%29))
  (bind _returnvalue (Transformation|GetActorLocation))
  (bind _path_point_array (Variables|Default|GetPath%20Point%20Array))
  (bind _curentpathindex (Variables|Default|GetCurentPathIndex))
  (bind _curentpathindex_2 (Variables|Default|GetCurentPathIndex))
  (bind _output (Utilities|Array|Get(acopy) _path_point_array _curentpathindex))
  ;[1 1 1] Move towards enemy.
  (if (Variables|Default|GetIs%20Grounded?)
    (Utilities|IsValid (Variables|Default|GetAs%20BP%20Enemy)
      (:Is%20Valid
        (Physics|AddForce (Variables|Default|GetSphere) (* (Math|Rotator|GetRotationXVector (Math|Rotator|FindLookatRotation _returnvalue _output)) 2.5e+03) "None" true)
        (if (Utilities|Operators|EqualEqual _returnvalue _output 5e+01)
          (Math|Integer|IncrementInt _curentpathindex_2
            (:%20%20
              (if (> _curentpathindex_2 (Utilities|Array|LastIndex (Variables|Default|GetPath%20Point%20Array)))
                _))))))))

(fn ConstructionScript)