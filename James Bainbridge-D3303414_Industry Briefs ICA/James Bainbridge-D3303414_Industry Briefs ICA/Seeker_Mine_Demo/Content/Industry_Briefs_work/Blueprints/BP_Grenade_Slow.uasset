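; BP_Grenade_Slow is a homing grenade that seeks enemies and bursts on contact; no slow effect is applied in this graph.
; DetectionField stores an overlapping BP_Enemy, and once a near-flat hit marks it grounded, Tick pushes Sphere toward that enemy.
; Trigger overlap with an enemy starts a delayed sparks-and-sound burst that hides and destroys the grenade.
; A BeginPlay timer also self-destructs it.
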(event OnComponentBeginOverlap(DetectionField)
  (params (OverlappedComponent :type Primitive%20Component%20Object%20Reference) (OtherActor :type Actor%20Object%20Reference) (OtherComp :type Primitive%20Component%20Object%20Reference) (OtherBodyIndex :type Integer) (bFromSweep :type Boolean) (SweepResult :type Hit%20Result%20Structure%20%28by%20ref%29))
  ;[1 1 1] Move towards enemy.
  (bind _asbp_enemy (Utilities|Casting|CastToBP_Enemy OtherActor))
  (Variables|Default|SetAs%20BP%20Enemy _asbp_enemy))

(event OnComponentHit(Sphere)
  (params (HitComponent :type Primitive%20Component%20Object%20Reference) (OtherActor :type Actor%20Object%20Reference) (OtherComp :type Primitive%20Component%20Object%20Reference) (NormalImpulse :type Vector :default "0, 0, 0") (Hit :type Hit%20Result%20Structure%20%28by%20ref%29))
  ;[1 1 1] Ground Detector
  (if (Utilities|Operators|EqualEqual (.ImpactNormal (Collision|BreakHitResult Hit)) "0.000000,0.000000,1.000000" 0.5)
    (Physics|SetSimulatePhysics (Variables|Default|GetGrenade) false)
    (Variables|Default|SetIs%20Grounded? true)
    (else
      (Variables|Default|SetIs%20Grounded? false))))

(event OnComponentBeginOverlap(Trigger)
  (params (OverlappedComponent :type Primitive%20Component%20Object%20Reference) (OtherActor :type Actor%20Object%20Reference) (OtherComp :type Primitive%20Component%20Object%20Reference) (OtherBodyIndex :type Integer) (bFromSweep :type Boolean) (SweepResult :type Hit%20Result%20Structure%20%28by%20ref%29))
  ;[1 1 1] Basics
  (Utilities|Casting|CastToBP_Enemy OtherActor)
  (CallFunction|DoStuff))

(event Custom|Do%20stuff
  ;[1 1 1] Basics
  (Variables|Default|SetExploded true)
  (Utilities|FlowControl|Delay 1.0)
  (Utilities|FlowControl|DoOnce false
    (:Completed
      (bind _returnvalue (Effects|SpawnEmitteratLocation "/Game/Everything_Else/StarterContent/Particles/P_Sparks.P_Sparks" (Transformation|GetActorLocation)))
      (Audio|PlaySoundatLocation "/Game/Everything_Else/StarterContent/Audio/Smoke01.Smoke01" (Transformation|GetActorLocation) "0, 0, 0" 1.0 1.0 0.0 0 0 0 0)
      (Development|SetHiddeninGame (Variables|Default|GetGrenade) true false)
      (Utilities|FlowControl|Delay 1.0)
      (Actor|DestroyActor)
      (Development|SetHiddeninGame _returnvalue true false))))

(event EventBeginPlay
  ;[1 1 1] Self-Destruct
  (Collision|SetCollisionEnabled (Variables|Default|GetFloorTrigger) "NoCollision")
  (if (not (Variables|Default|GetExploded))
    (Utilities|FlowControl|Delay 1e+01)
    (Actor|DestroyActor)))

(event EventTick
  (params (DeltaSeconds :type Float%20%28single-precision%29))
  ;[1 1 1] Move towards enemy.
  (if (Variables|Default|GetIs%20Grounded?)
    (Utilities|IsValid (Variables|Default|GetAs%20BP%20Enemy)
      (:Is%20Valid
        (Physics|AddForce (Variables|Default|GetSphere) (* (Math|Rotator|GetRotationXVector (Math|Rotator|FindLookatRotation (Transformation|GetActorLocation) (Transformation|GetActorLocation (Variables|Default|GetAs%20BP%20Enemy)))) 1e+03) "None" true)))))

(fn ConstructionScript)